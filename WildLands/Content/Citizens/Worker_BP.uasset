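; Worker_BP is a citizen worker actor that shows its work progress through a progress bar widget component.
; On BeginPlay it caches the component's ProgressBar_BP widget and binds UpdateBar to an update event.
; Each update shows the bar while Working, hides it while Waiting for Work, and passes BarPercent to the widget, with no Tick logic.
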(event Custom|UpdateBar
  (bind _progressbar (Variables|Default|GetProgressBar))
  (switch Utilities|FlowControl|Switch|SwitchonEWorkerStatus (Variables|Default|GetWorkerStatus)
    (:WaitingForWork
      (Rendering|SetVisibility _progressbar false true))
    (:Working
      (Rendering|SetVisibility _progressbar true true)))
  (Default|Update% (stale EventBeginPlay _output_get) (Variables|Default|GetBarPercent)))

(event EventBeginPlay
  (bind _asprogress_bar_bp (Utilities|Casting|CastToProgressBar_BP (UserInterface|GetUserWidgetObject (Variables|Default|GetProgressBar))))
  (bind _output_get (Variables|Default|SetProgressBarWidgetRef _asprogress_bar_bp))
  (EventDispatchers|BindEventtoUpdateProgressBar (delegate Custom|UpdateBar)))

(event Collision|EventActorBeginOverlap
  (params (OtherActor :type Actor%20Object%20Reference)))

(event EventTick
  (params (DeltaSeconds :type Float%20%28single-precision%29)))

(fn ConstructionScript)